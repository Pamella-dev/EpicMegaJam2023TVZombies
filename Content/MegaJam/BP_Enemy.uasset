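; Enemy character for a game jam project that wanders the navmesh and chases pawns it sees.
; Wandering chains AI MoveTo calls to random reachable points around its current location.
; PawnSensing sightings start a chase, with a DoOnce switching to sprint speed and replaying a looping animation once.
; A retriggerable delay restores walk speed, resets the sprint gate and resumes wandering shortly after sightings stop.
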(event `self.ReceiveBeginPlay`
  ;[1 1 1] Pick Random Locaton
  (`self.MoveToRandomLocation`))

(event `MoveToRandomLocation`
  ;[1 1 1] Pick Random Locaton
  (bind _randomlocation (`NavigationSystemV1.K2_GetRandomLocationInNavigableRadius` (`self.K2_GetActorLocation`) 1000.0 null null))
  (`|AIMoveTo` self _randomlocation null
    (:`OnSuccess`
      (`self.MoveToRandomLocation`))))

(event `CanSprintAgain`
  ;[1 1 1] Chase (NEED TO PUT THE CORRECT ANIM)
  (goto _label :!via `Reset`))

(event `self.PawnSensing.OnSeePawn`
  (params (Pawn :type "Pawn Object Reference"))
  ;[1 1 1] Chase (NEED TO PUT THE CORRECT ANIM)
  (`|ExecutionSequence`
    (:`then_0`
      (`/Engine/EditorBlueprintResources/StandardMacros.DoOnce` false :!label _label
        (:`Completed`
          (`SkeletalMeshComponent.PlayAnimation` (`self.Mesh`) null true)
          (set `CharacterMovementComponent.MaxWalkSpeed` 400.0 (`self.CharacterMovement`)))))
    (:`then_1`
      (`|AIMoveTo` self (0.0 0.0 0.0) Pawn
        (:`then`
          (`KismetSystemLibrary.RetriggerableDelay` 2.0)
          (`SkeletalMeshComponent.PlayAnimation` (`self.Mesh`) null true)
          (set `CharacterMovementComponent.MaxWalkSpeed` 200.0 (`self.CharacterMovement`))
          (`self.CanSprintAgain`)
          (`self.MoveToRandomLocation`))))))

(fn `UserConstructionScript`)