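; BP_End is the game's exit trigger, quitting the game when an actor overlaps it after all tapes have been collected.
; On BeginPlay it caches the player's BP_ThirdPersonCharacter.
; Each Tick it polls that character's TapeCounter and sets AllTapesTaken once five tapes are counted.
; The overlap event only checks that flag, not which actor entered.
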(event `self.ReceiveBeginPlay`
  ;[1 1 1] Variable From Character
  (bind _asbp_third_person_character (cast `/Game/ThirdPerson/Blueprints/BP_ThirdPersonCharacter` (`GameplayStatics.GetPlayerCharacter` 0)))
  (set `self.As BP Third Person Character` _asbp_third_person_character))

(event `self.ReceiveActorBeginOverlap`
  (params (OtherActor :type "Actor Object Reference"))
  ;[1 1 1] The End
  (if (`self.AllTapesTaken?`)
    (`KismetSystemLibrary.QuitGame` null "Quit")))

(event `self.ReceiveTick`
  (params (DeltaSeconds :type "Float (single-precision)"))
  ;[1 1 1] All Tapes Taken is True?
  (if (== (`/Game/ThirdPerson/Blueprints/BP_ThirdPersonCharacter.TapeCounter` (`self.As BP Third Person Character`)) 5)
    (set `self.AllTapesTaken?` true)))

(fn `UserConstructionScript`)